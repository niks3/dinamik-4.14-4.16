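; Homing projectile Blueprint that seeks and damages a girl character (Exp_devojcia).
; On BeginPlay it sets the capsule of the first Exp_devojcia1 actor found as the ProjectileMovement homing target.
; A capsule overlap that casts to exp_devojcia applies fixed damage through DmgSistem, stops movement and disables collision responses.
; The hit also sets the Umro flag, plays a camera shake and hurt vocal, then destroys the projectile after a short delay.
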(event `self.ReceiveBeginPlay`
  (`|ExecutionSequence`
    (:`then_0`
      (bind _outactors (`GameplayStatics.GetAllActorsOfClass` "/Game/purgatorium/Menu/testis2/Aseti_final/exp_devojcia1.exp_devojcia1_C"))
      (set `ProjectileMovementComponent.HomingTargetComponent` (`Character.CapsuleComponent` (`KismetArrayLibrary.Array_Get` _outactors)) (`self.ProjectileMovement`)))))

(event `self.Capsule.OnComponentBeginOverlap`
  (params (OverlappedComponent :type "PrimitiveComponent Object Reference") (OtherActor :type "Actor Object Reference") (OtherComp :type "PrimitiveComponent Object Reference") (OtherBodyIndex :type Integer) (bFromSweep :type Boolean) (SweepResult :type "HitResult Structure (by ref)"))
  (`|ExecutionSequence`
    (:`then_0`
      (bind _asexp_devojcia (cast `/Game/purgatorium/Menu/testis2/Aseti_final/exp_devojcia` OtherActor))
      (`/Game/purgatorium/Menu/testis2/Aseti_final/exp_devojcia.dmg sistem` _asexp_devojcia 0.201)
      (`MovementComponent.StopMovementImmediately` (`self.ProjectileMovement`))
      (set `self.umro` true)
      (`PrimitiveComponent.SetCollisionResponseToAllChannels` (`self.Capsule`) "ECR_Ignore")
      (`GameplayStatics.PlayWorldCameraShake` "/Game/purgatorium/bluprint/props/trzaj_kamere.trzaj_kamere_C" (`SceneComponent.K2_GetComponentLocation` (`self.Capsule`)) 0.0 100000000.0)
      (`GameplayStatics.PlaySound2D` "/Game/purgatorium/zvuk/DMG_vocal_Cue.DMG_vocal_Cue")
      (`KismetSystemLibrary.Delay` 0.2)
      (`self.K2_DestroyActor`))))

(fn `UserConstructionScript`)