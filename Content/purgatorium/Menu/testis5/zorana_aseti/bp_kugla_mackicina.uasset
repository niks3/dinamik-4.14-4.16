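; Homing projectile actor that breaks destructible box_dest_zorana objects on contact.
; On BeginPlay it sets the first Bp_mackica's Scene component as the ProjectileMovement homing target.
; When Sphere1 overlaps a box, it applies destructible damage with an impulse along X, stops moving, disables flipbook collision and plays a world camera shake.
; The projectile destroys itself after a short delay.
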(event `self.ReceiveBeginPlay`
  (`|ExecutionSequence`
    (:`then_0`
      (bind _outactors (`GameplayStatics.GetAllActorsOfClass` "/Game/purgatorium/Menu/testis5/zorana_aseti/bp_mackica.bp_mackica_C"))
      (set `ProjectileMovementComponent.HomingTargetComponent` (`/Game/purgatorium/Menu/testis5/zorana_aseti/bp_mackica.Scene` (`KismetArrayLibrary.Array_Get` _outactors)) (`self.ProjectileMovement`)))))

(event `self.Sphere1.OnComponentBeginOverlap`
  (params (OverlappedComponent :type "PrimitiveComponent Object Reference") (OtherActor :type "Actor Object Reference") (OtherComp :type "PrimitiveComponent Object Reference") (OtherBodyIndex :type Integer) (bFromSweep :type Boolean) (SweepResult :type "HitResult Structure (by ref)"))
  (bind _paperflipbook (`self.PaperFlipbook`))
  (bind _asbox_dest_zorana (cast `/Game/purgatorium/Menu/testis5/zorana_aseti/box_dest_zorana` OtherActor))
  (`DestructibleComponent.ApplyDamage` (`/Game/purgatorium/Menu/testis5/zorana_aseti/box_dest_zorana.Destructible` _asbox_dest_zorana) 1.0 (`SceneComponent.K2_GetComponentLocation` (`self.PaperFlipbook`)) (1.0 0.0 0.0) 40000.0)
  (`MovementComponent.StopMovementImmediately` (`self.ProjectileMovement`))
  (`PrimitiveComponent.SetCollisionResponseToAllChannels` _paperflipbook "ECR_Ignore")
  (`GameplayStatics.PlayWorldCameraShake` "/Game/purgatorium/bluprint/props/trzaj_kamere.trzaj_kamere_C" (`SceneComponent.K2_GetComponentLocation` _paperflipbook) 0.0 100000000.0)
  (`KismetSystemLibrary.Delay` 0.2)
  (`self.K2_DestroyActor`))

(fn `UserConstructionScript`)