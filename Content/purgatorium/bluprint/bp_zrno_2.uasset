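; Projectile Blueprint with a Paper2D flipbook that damages or reacts to specific actor classes it hits.
; Box overlap runs a Sequence of casts, calling damage functions on characters and exp_krava, or applying impulse damage to box_dest using bp_kain's cast result for direction.
; Most hits show a blood flipbook, stop movement, disable collision, shake the camera and destroy after a delay.
; Plant, knife and fist hits show a bullet-burst flipbook before destruction.
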(event `self.Box.OnComponentBeginOverlap`
  (params (OverlappedComponent :type "PrimitiveComponent Object Reference") (OtherActor :type "Actor Object Reference") (OtherComp :type "PrimitiveComponent Object Reference") (OtherBodyIndex :type Integer) (bFromSweep :type Boolean) (SweepResult :type "HitResult Structure (by ref)"))
  (`|ExecutionSequence`
    (:`then_0`
      (bind _asbp_lik (cast `/Game/purgatorium/bluprint/bp_lik` OtherActor))
      (`/Game/purgatorium/bluprint/bp_lik.DMG_sistem_mele` _asbp_lik (`self.dmgValue`))
      (`PaperFlipbookComponent.SetFlipbook` (`self.PaperFlipbook`) "/Game/purgatorium/sprajtovi/Art/krv/pucanj_-_krv.pucanj_-_krv")
      (`MovementComponent.StopMovementImmediately` (`self.ProjectileMovement`) :!label _label)
      (`PrimitiveComponent.SetCollisionResponseToAllChannels` (`self.Box`) "ECR_Ignore")
      (`GameplayStatics.PlayWorldCameraShake` "/Game/purgatorium/bluprint/props/trzaj_kamere.trzaj_kamere_C" (`SceneComponent.K2_GetComponentLocation` (`self.Box`)) 0.0 100000000.0)
      (`KismetSystemLibrary.Delay` 0.2)
      (`self.K2_DestroyActor`))
    (:`then_1`
      (bind _asbp_kain (cast `/Game/purgatorium/bluprint/bp_kain` OtherActor))
      (`/Game/purgatorium/bluprint/bp_kain.dmg sistem` _asbp_kain (`self.dmgValue`))
      (`PaperFlipbookComponent.SetFlipbook` (`self.PaperFlipbook`) "/Game/purgatorium/sprajtovi/Art/krv/pucanj_-_krv.pucanj_-_krv")
      (goto _label))
    (:`then_2`
      (cast `/Game/purgatorium/bluprint/bp_zrno` OtherActor)
      (`PaperFlipbookComponent.SetFlipbook` (`self.PaperFlipbook`) "/Game/purgatorium/sprajtovi/Art/krv/pucanj_-_krv.pucanj_-_krv")
      (goto _label))
    (:`then_3`
      (cast `/Game/purgatorium/bluprint/kolajder` OtherActor)
      (`PaperFlipbookComponent.SetFlipbook` (`self.PaperFlipbook`) "/Game/purgatorium/sprajtovi/Art/krv/pucanj_-_krv.pucanj_-_krv")
      (goto _label))
    (:`then_4`
      (cast `/Game/purgatorium/bluprint/bp_Biljka` OtherActor)
      (`PaperFlipbookComponent.SetFlipbook` (`self.PaperFlipbook`) "/Game/purgatorium/sprajtovi/Art/pucanje/pucanje_metka.pucanje_metka")
      (`KismetSystemLibrary.Delay` 0.12)
      (`self.K2_DestroyActor`))
    (:`then_5`
      (cast `/Game/purgatorium/bluprint/bp_noz` OtherActor)
      (`PaperFlipbookComponent.SetFlipbook` (`self.PaperFlipbook`) "/Game/purgatorium/sprajtovi/Art/pucanje/pucanje_metka.pucanje_metka")
      (`KismetSystemLibrary.Delay` 0.12)
      (`self.K2_DestroyActor`)
      (goto _label))
    (:`then_6`
      (cast `/Game/purgatorium/bluprint/bp_saka` OtherActor)
      (`PaperFlipbookComponent.SetFlipbook` (`self.PaperFlipbook`) "/Game/purgatorium/sprajtovi/Art/pucanje/pucanje_metka.pucanje_metka")
      (`KismetSystemLibrary.Delay` 0.12)
      (`self.K2_DestroyActor`))
    (:`then_7`
      (cast `/Game/purgatorium/bluprint/props/bp_ptica` OtherActor)
      (`PaperFlipbookComponent.SetFlipbook` (`self.PaperFlipbook`) "/Game/purgatorium/sprajtovi/Art/krv/pucanj_-_krv.pucanj_-_krv")
      (goto _label))
    (:`then_8`
      (bind _asbp_kain_sake (cast `/Game/purgatorium/bluprint/bp_kainSake` OtherActor))
      (`/Game/purgatorium/bluprint/bp_kainSake.dmg sistem` _asbp_kain_sake (`self.dmgValue`))
      (`PaperFlipbookComponent.SetFlipbook` (`self.PaperFlipbook`) "/Game/purgatorium/sprajtovi/Art/krv/pucanj_-_krv.pucanj_-_krv")
      (goto _label))
    (:`then_9`
      (bind _asexp_krava (cast `/Game/purgatorium/bluprint/exp_krava` OtherActor))
      (`/Game/purgatorium/bluprint/exp_krava.dmg sistem` _asexp_krava 0.1)
      (`PaperFlipbookComponent.SetFlipbook` (`self.PaperFlipbook`) "/Game/purgatorium/sprajtovi/Art/krv/pucanj_-_krv.pucanj_-_krv")
      (goto _label))
    (:`then_10`
      (cast `/Game/purgatorium/bluprint/exp_kugla` OtherActor)
      (`PaperFlipbookComponent.SetFlipbook` (`self.PaperFlipbook`) "/Game/purgatorium/sprajtovi/Art/krv/pucanj_-_krv.pucanj_-_krv")
      (goto _label))
    (:`then_11`
      (bind _asbox_dest (cast `/Game/purgatorium/Menu/testis1/aseti_lv2/box_dest` OtherActor))
      (`DestructibleComponent.ApplyDamage` (`/Game/purgatorium/Menu/testis1/aseti_lv2/box_dest.Destructible` _asbox_dest) 1.0 (`SceneComponent.K2_GetComponentLocation` (`self.Box`)) (`KismetMathLibrary.MakeVector` (`KismetMathLibrary.Conv_IntToDouble` (`/Game/purgatorium/bluprint/bp_kain.pravac` _asbp_kain)) 0.0) 40000.0)
      (`PaperFlipbookComponent.SetFlipbook` (`self.PaperFlipbook`) "/Game/purgatorium/sprajtovi/Art/krv/pucanj_-_krv.pucanj_-_krv")
      (`MovementComponent.StopMovementImmediately` (`self.ProjectileMovement`))
      (`PrimitiveComponent.SetCollisionResponseToAllChannels` (`self.Box`) "ECR_Ignore")
      (`GameplayStatics.PlayWorldCameraShake` "/Game/purgatorium/bluprint/props/trzaj_kamere.trzaj_kamere_C" (`SceneComponent.K2_GetComponentLocation` (`self.Box`)) 0.0 100000000.0)
      (`KismetSystemLibrary.Delay` 0.2)
      (`self.K2_DestroyActor`))))

(fn `UserConstructionScript`)