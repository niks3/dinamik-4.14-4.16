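; Dynamic collider prop that shuttles back and forth along the world X axis between two hardcoded bounds.
; Each Tick checks the root's X position and, beyond either bound, zeroes the ProjectileMovement velocity.
; A short Delay then sends it at constant speed in the opposite direction, producing a pause at each end.
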(event `self.ReceiveTick`
  (params (DeltaSeconds :type "Float (single-precision)"))
  (bind _returnvalue_x (`KismetMathLibrary.BreakVector` (`SceneComponent.K2_GetComponentLocation` (`self.root`))))
  (if (<= _returnvalue_x 3000.0)
    (if (<= _returnvalue_x -2000.0)
      (set `MovementComponent.Velocity` (0.0 0.0 0.0) (`self.ProjectileMovement`))
      (`KismetSystemLibrary.Delay` 2.0)
      (set `MovementComponent.Velocity` (2000.0 0.0 0.0) (`self.ProjectileMovement`)))
    (else
      (set `MovementComponent.Velocity` (0.0 0.0 0.0) (`self.ProjectileMovement`))
      (`KismetSystemLibrary.Delay` 2.0)
      (set `MovementComponent.Velocity` (-2000.0 0.0 0.0) (`self.ProjectileMovement`)))))

(fn `UserConstructionScript`)