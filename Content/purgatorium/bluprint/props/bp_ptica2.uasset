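; A Paper2D bird prop ("ptica") that flies back and forth along the X axis and is destroyed by grain ("zrno") actors.
; Tick checks the root's world X against two fixed bounds and reverses the ProjectileMovement velocity outside them.
; Overlapping any of four grain Blueprint classes swaps the flipbook to a smoke animation, zeroes the velocity and destroys the bird after a short delay.
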(event `self.PaperFlipbook.OnComponentBeginOverlap`
  (params (OverlappedComponent :type "PrimitiveComponent Object Reference") (OtherActor :type "Actor Object Reference") (OtherComp :type "PrimitiveComponent Object Reference") (OtherBodyIndex :type Integer) (bFromSweep :type Boolean) (SweepResult :type "HitResult Structure (by ref)"))
  (`|ExecutionSequence`
    (:`then_0`
      (cast `/Game/purgatorium/bluprint/bp_zrno` OtherActor))
    (:`then_1`
      (cast `/Game/purgatorium/bluprint/bp_zrno_2` OtherActor))
    (:`then_2`
      (cast `/Game/purgatorium/bluprint/bp_zrno_po_zedu` OtherActor))
    (:`then_3`
      (cast `/Game/purgatorium/bluprint/bp_zrno_po_zedu_2` OtherActor)))
  (`PaperFlipbookComponent.SetFlipbook` (`self.PaperFlipbook`) "/Game/purgatorium/sprajtovi/Art/prasina_skok/karakter_-_skok_-_dim_na_podu.karakter_-_skok_-_dim_na_podu")
  (set `MovementComponent.Velocity` (0.0 0.0 0.0) (`self.ProjectileMovement`))
  (`KismetSystemLibrary.Delay` 0.5)
  (`self.K2_DestroyActor`))

(event `self.ReceiveTick`
  (params (DeltaSeconds :type "Float (single-precision)"))
  (bind _returnvalue_x (`KismetMathLibrary.BreakVector` (`SceneComponent.K2_GetComponentLocation` (`self.root`))))
  (if (<= _returnvalue_x 3000.0)
    (if (<= _returnvalue_x -2200.0)
      (set `MovementComponent.Velocity` (1000.0 0.0 0.0) (`self.ProjectileMovement`)))
    (else
      (set `MovementComponent.Velocity` (-1000.0 0.0 0.0) (`self.ProjectileMovement`)))))

(fn `UserConstructionScript`)