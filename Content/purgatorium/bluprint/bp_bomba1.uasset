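; bp_bomba1 is a bomb actor that damages a bp_lik on contact and then destroys itself.
; Its Box overlap runs a sequence of class casts, passing DmgValue to DmgSistem on bp_lik.
; Overlaps with several other classes, such as kolajder, bp_Biljka and bp_ptica, destroy the bomb without dealing damage.
; A similar damage branch for bp_kain is left unconnected and never runs.
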(event `self.Box.OnComponentBeginOverlap`
  (params (OverlappedComponent :type "PrimitiveComponent Object Reference") (OtherActor :type "Actor Object Reference") (OtherComp :type "PrimitiveComponent Object Reference") (OtherBodyIndex :type Integer) (bFromSweep :type Boolean) (SweepResult :type "HitResult Structure (by ref)"))
  (`|ExecutionSequence`
    (:`then_0`
      (bind _asbp_lik (cast `/Game/purgatorium/bluprint/bp_lik` OtherActor))
      (`/Game/purgatorium/bluprint/bp_lik.dmg sistem` _asbp_lik (`self.dmgValue`))
      (`self.K2_DestroyActor`))
    (:`then_2`
      (cast `/Game/purgatorium/bluprint/bp_zrno_2` OtherActor)
      (`self.K2_DestroyActor`))
    (:`then_3`
      (cast `/Game/purgatorium/bluprint/kolajder` OtherActor)
      (`self.K2_DestroyActor` :!label _label))
    (:`then_4`
      (cast `/Game/purgatorium/bluprint/bp_Biljka` OtherActor)
      (goto _label))
    (:`then_5`
      (cast `/Game/purgatorium/bluprint/bp_zamka5` OtherActor)
      (goto _label))
    (:`then_6`
      (cast `/Game/purgatorium/bluprint/bp_saka` OtherActor)
      (goto _label))
    (:`then_7`
      (cast `/Game/purgatorium/bluprint/props/bp_ptica` OtherActor)
      (goto _label))))

(fn `UserConstructionScript`)