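; A homing shuriken projectile with a Paper2D flipbook that damages the player-type characters it hits.
; On BeginPlay its ProjectileMovement homes on the capsule of the first Exp_devojcia actor found in the level.
; When its sphere overlaps an exp_devojcia or exp_devojcia1, it calls that actor's DmgSistem, stops, switches to a smoke flipbook, plays a damage sound and destroys itself after a short delay.
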(event `self.ReceiveBeginPlay`
  (bind _outactors (`GameplayStatics.GetAllActorsOfClass` "/Game/purgatorium/Menu/testis2/Aseti_final/exp_devojcia.exp_devojcia_C"))
  (set `ProjectileMovementComponent.HomingTargetComponent` (`Character.CapsuleComponent` (`KismetArrayLibrary.Array_Get` _outactors)) (`self.ProjectileMovement`)))

(event `self.Sphere.OnComponentBeginOverlap`
  (params (OverlappedComponent :type "PrimitiveComponent Object Reference") (OtherActor :type "Actor Object Reference") (OtherComp :type "PrimitiveComponent Object Reference") (OtherBodyIndex :type Integer) (bFromSweep :type Boolean) (SweepResult :type "HitResult Structure (by ref)"))
  (`|ExecutionSequence`
    (:`then_1`
      (bind _asexp_devojcia_1 (cast `/Game/purgatorium/Menu/testis2/Aseti_final/exp_devojcia1` OtherActor))
      (`/Game/purgatorium/Menu/testis2/Aseti_final/exp_devojcia1.dmg sistem` _asexp_devojcia_1 0.201))
    (:`then_2`
      (bind _asexp_devojcia (cast `/Game/purgatorium/Menu/testis2/Aseti_final/exp_devojcia` OtherActor))
      (`/Game/purgatorium/Menu/testis2/Aseti_final/exp_devojcia.dmg sistem` _asexp_devojcia 0.201)))
  (`MovementComponent.StopMovementImmediately` (`self.ProjectileMovement`))
  (`PaperFlipbookComponent.SetFlipbook` (`self.PaperFlipbook`) "/Game/purgatorium/sprajtovi/Art/prasina_skok/karakter_-_skok_-_dim_na_podu.karakter_-_skok_-_dim_na_podu")
  (`GameplayStatics.PlaySound2D` "/Game/purgatorium/zvuk/DMG_vocal_Cue.DMG_vocal_Cue")
  (`KismetSystemLibrary.Delay` 0.4)
  (`self.K2_DestroyActor`))

(fn `UserConstructionScript`)